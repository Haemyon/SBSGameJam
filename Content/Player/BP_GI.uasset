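; Game instance Blueprint that handles network and travel failures and leaving a multiplayer session.
; Network and travel error events print the failure type to screen, then share one DestroySession call for player controller 0.
; LeaveSession opens the main menu level, then destroys the session.
; Init and Shutdown are empty.
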(event Custom|LeaveSession
  ;[1 1 1] 세션 떠나기
  (Game|OpenLevel(byName) "MainMenu_Level")
  (|DestroySession (Game|GetPlayerController 0)))

(event EventShutdown)

(event EventInit)

(event EventHandleNetworkError
  (params (FailureType :type ENetworkFailure%20Enum :default "NetDriverAlreadyExists") (bIsServer :type Boolean))
  ;[1 1 1] 네트워크 및 트래블 에러
  (Development|PrintString (Utilities|String|EnumtoString FailureType))
  (|DestroySession (Game|GetPlayerController 0)))

(event EventHandleTravelError
  (params (FailureType :type ETravelFailure%20Enum :default "NoLevel"))
  ;[1 1 1] 네트워크 및 트래블 에러
  (Development|PrintString (Utilities|String|EnumtoString FailureType))
  (|DestroySession (Game|GetPlayerController 0)))