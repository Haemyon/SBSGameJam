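; BP_PC_Core is a player controller that opens and closes the in-game menu on the IA_GameMenu input.
; ToggleGameMenu creates WB_GameMenu and adds it to the viewport on first use, then reuses that instance by switching it between visible and collapsed.
; FocusWidget and FocusGame switch the mouse cursor and input mode to match the menu state, and play begins in game-only input.
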(event Input|EnhancedActionEvents|EnhancedInputActionIA_GameMenu
  (params (ActionValue :type Boolean) (ElapsedSeconds :type Float%20%28double-precision%29) (TriggeredSeconds :type Float%20%28double-precision%29) (InputAction :type Input%20Action%20Object%20Reference :default "/Game/Player/Input/IA_GameMenu.IA_GameMenu"))
  (:Started
    (Widget|ToggleGameMenu)))

(event EventBeginPlay
  (Input|SetInputModeGameOnly self false))

(fn ConstructionScript)

(fn FocusWidget
  (Variables|Default|SetbShowMouseCursor true)
  (Input|SetInputModeGameandUI self (Variables|Default|GetWB_GameMenu) "DoNotLock" true false))

(fn FocusGame
  (Variables|Default|SetbShowMouseCursor false)
  (Input|SetInputModeGameOnly self false))

(fn ToggleGameMenu
  (Variables|Default|GetWB_GameMenu
    (:then
      (if (Widget|IsVisible (Variables|Default|GetWB_GameMenu))
        (Widget|SetVisibility (Variables|Default|GetWB_GameMenu) "Collapsed")
        (Widget|FocusGame)
        (else
          (Widget|SetVisibility (Variables|Default|GetWB_GameMenu) "Visible")
          (Widget|FocusWidget))))
    (:else
      (bind _returnvalue (UserInterface|CreateWidget "/Game/Widget/GamePlay/WB_GameMenu.WB_GameMenu_C" self))
      (bind _output_get (Variables|Default|SetWB_GameMenu _returnvalue))
      (UserInterface|Viewport|AddtoViewport _output_get 0)
      (Widget|FocusWidget))))