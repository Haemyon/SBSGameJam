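; Player character Blueprint that handles interaction, item pickup and equipping a held weapon.
; Interact input passes the current InteractionActor to Hand, which sends it an interface message with the character, while primary action input fires the OnPrimaryAction dispatcher.
; HandlePickUp stores the item ID in CurrentWeapon, whose RepNotify looks up the DT_Item row, swaps the Handleing child actor class and runs SetupWeapon.
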(event Custom|Hand
  (params (타깃 :type Object%20Object%20Reference))
  (Class|BPIInteraction|HandInteract(Message) 타깃 self))

(event Input|EnhancedActionEvents|EnhancedInputActionIA_Interact
  (params (ActionValue :type Boolean) (ElapsedSeconds :type Float%20%28double-precision%29) (TriggeredSeconds :type Float%20%28double-precision%29) (InputAction :type Input%20Action%20Object%20Reference :default "/Game/Player/Input/IA_Interact.IA_Interact"))
  (:Started
    (CallFunction|Hand (Variables|Default|GetInteractionActor))))

(event Input|EnhancedActionEvents|EnhancedInputActionIA_PrimaryAction
  (params (ActionValue :type Boolean) (ElapsedSeconds :type Float%20%28double-precision%29) (TriggeredSeconds :type Float%20%28double-precision%29) (InputAction :type Input%20Action%20Object%20Reference :default "/Game/Player/Input/IA_PrimaryAction.IA_PrimaryAction"))
  (:Started
    (Default|CallOnPrimaryAction)))

(event EventBeginPlay
  (|CallParentFunction))

(event EventHandlePickUp
  (params (ID :type String))
  (Variables|Default|SetCurrentWeapon ID))

(fn ConstructionScript
  (|CallParentFunction))

(fn OnRepCurrentWeapon0
  (bind _returnvalue (Utilities|GetDataTableRow "/Game/Blueprint/DATA/DT_Item.DT_Item" (Utilities|String|StringToName (Variables|Default|GetCurrentWeapon)))
    (:then
      (ChildActorComponent|SetChildActorClass (Variables|Default|GetHandleing) (.Blueprint (Utilities|Struct|BreakS_Item _returnvalue)))
      (CallFunction|SetupWeapon))))