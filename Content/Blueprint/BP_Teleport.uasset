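; BP_Teleport is an actor that gathers every BP_CoreCharacter around its Box component, apparently as a start point.
; StartTeleport runs only with authority, stores the actor's location in TeleportLocation and calls SpawnStartPoint.
; SpawnStartPoint teleports each character without sweep to a random point in a small fixed-size volume centred on the Box, independent of its extent.
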(event Custom|StartTeleport
  (Networking|SwitchHasAuthority
    (:Authority
      (Variables|Default|SetTeleportLocation (Transformation|GetActorLocation))
      (CallFunction|SpawnStartPoint))))

(fn ConstructionScript)

(fn SpawnStartPoint
  (bind _outactors (Actor|GetAllActorsOfClass "/Game/Player/BP_CoreCharacter.BP_CoreCharacter_C"))
  (for _array_element _outactors
    (Transformation|SetActorLocation _array_element (Math|Random|RandomPointinBoundingBox (Transformation|GetWorldLocation (Variables|Default|GetBox)) "32.000000,32.000000,32.000000") false true)))