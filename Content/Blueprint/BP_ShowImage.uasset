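; BP_ShowImage is an interactable actor with a prompt widget, apparently meant to show an image, though that logic is disconnected.
; BeginPlay passes InteractName to the prompt, and SetFocused shows it, using a retriggerable delay to hide it once focus calls stop.
; IsTurn's RepNotify calls an empty TurnActor event.
; The cube-rotation timeline and the temporary WB_ShowImage popup are never executed.
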(event Custom|TurnActor)

(event Custom|Reset%20Boolean
  (Variables|Default|SetIsTurn? false))

(event EventSetFocused
  (Rendering|SetVisibility (Variables|Default|GetWidget) true false)
  (Utilities|FlowControl|RetriggerableDelay 0.1)
  (Rendering|SetVisibility (Variables|Default|GetWidget) false false))

(event EventBeginPlay
  (CallFunction|SetupInteractionWidget))

(fn ConstructionScript)

(fn SetupInteractionWidget
  (bind _aswb_interaction_feed_back (Utilities|Casting|CastToWB_InteractionFeedBack (UserInterface|GetWidget (Variables|Default|GetWidget))))
  (Default|UpdateWidget _aswb_interaction_feed_back (Variables|Default|GetInteract_Name)))

(fn OnRepIsTurn?
  (CallFunction|TurnActor))