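; BP_EndPoint is a level end trigger that detects when enough players gather in its Box volume.
; Box overlap begin increments PlayerCount and end decrements it, printing the count on entry.
; Once the count reaches four, it calls EndingPointMessage on the GameState.
; Overlaps are counted without filtering the overlapping actor type.
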(event OnComponentBeginOverlap(Box)
  (params (OverlappedComponent :type Primitive%20Component%20Object%20Reference) (OtherActor :type Actor%20Object%20Reference) (OtherComp :type Primitive%20Component%20Object%20Reference) (OtherBodyIndex :type Integer) (bFromSweep :type Boolean) (SweepResult :type Hit%20Result%20Structure%20%28by%20ref%29))
  (bind _result (Math|Float|IncrementFloat (Variables|Default|GetPlayerCount))
    (:%20%20
      (bind _output_get (Variables|Default|SetPlayerCount _result))
      (Development|PrintString (Utilities|String|ToString(Float) _output_get))
      (if (>= (Variables|Default|GetPlayerCount) 4.0)
        (Class|BPIGameState|EndingPoint(Message) (Game|GetGameState))))))

(event OnComponentEndOverlap(Box)
  (params (OverlappedComponent :type Primitive%20Component%20Object%20Reference) (OtherActor :type Actor%20Object%20Reference) (OtherComp :type Primitive%20Component%20Object%20Reference) (OtherBodyIndex :type Integer))
  (bind _result (Math|Float|DecrementFloat (Variables|Default|GetPlayerCount))
    (:%20%20
      (Variables|Default|SetPlayerCount _result))))

(fn ConstructionScript)