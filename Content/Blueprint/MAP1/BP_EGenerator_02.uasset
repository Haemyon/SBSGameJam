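; BP_EGenerator_02 is an interactable generator that opens the way by triggering every BP_Door03 once it holds three blue batteries.
; AddCount_Blue increments the battery count and refreshes the WB_InteractionFeedBack widget, which shows the Korean battery label with progress out of three.
; SetFocused shows that widget and uses a retriggerable delay to hide it shortly after focus stops.
; Interact checks the count and uses IsTurn to fire the doors' FunctionInteract only once.
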(event Custom|AddCount_Blue
  (bind _result (Math|Float|IncrementFloat (Variables|Default|GetBlue_BatteryCount))
    (:%20%20
      (Development|PrintString (Utilities|String|ToString(Float) _result) true true "(R=0.000000,G=0.259845,B=1.000000,A=1.000000)" 1e+01)
      (CallFunction|SetupInteractionWidget))))

(event EventFunctionInteract)

(event EventSetFocused
  (Rendering|SetVisibility (Variables|Default|GetWidget) true false)
  (Utilities|FlowControl|RetriggerableDelay 0.1)
  (Rendering|SetVisibility (Variables|Default|GetWidget) false false))

(event EventBeginPlay
  (CallFunction|SetupInteractionWidget))

(event EventInteract
  (params (InteractingActor :type Actor%20Object%20Reference))
  (if (>= (Variables|Default|GetBlue_BatteryCount) 3.0)
    (Development|PrintString "Blue Compelete")
    (if (not (Variables|Default|GetIs%20Turn?))
      (Variables|Default|SetIs%20Turn? true)
      (bind _outactors (Actor|GetAllActorsOfClass "/Game/Blueprint/MAP1/BP_Door03.BP_Door03_C"))
      (for _array_element _outactors
        (Default|FunctionInteract _array_element)))))

(fn ConstructionScript)

(fn SetupInteractionWidget
  (bind _aswb_interaction_feed_back (Utilities|Casting|CastToWB_InteractionFeedBack (UserInterface|GetWidget (Variables|Default|GetWidget))))
  (Default|UpdateWidget _aswb_interaction_feed_back (Utilities|Text|ToText(String) (Utilities|String|Append " 배터리 " (Utilities|String|ToString(Integer) (Math|Float|Round (Variables|Default|GetBlue_BatteryCount))) "/3"))))

(fn OnRepBlueBatteryCount)