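; BP_Door01 is an interactable door that slides open once, with no logic to close it.
; FunctionInteract sets IsTurn, whose RepNotify plays the Turn timeline, adding its Z value to the Cube's relative X on each update.
; SetFocused shows the interaction widget and hides it through a 0.1-second retriggerable delay, so it stays visible while focus repeats.
; BeginPlay optionally fills that widget with InteractName.
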(event Custom|TurnActor
  (bind _cube (Variables|Default|GetCube))
  (bind _relativelocation (Variables|/Script/Engine.SceneComponent|GetRelativeLocation _cube))
  (bind _z (Timeline|Turn PlayFromStart)
    (:Update
      (Transformation|SetRelativeLocation _cube (Math|Vector|MakeVector (+ (.x _relativelocation) _z) (.y _relativelocation) (.z _relativelocation)) false false))))

(event EventFunctionInteract
  (if (not (Variables|Default|GetIsTurn?))
    (Variables|Default|SetIsTurn? true)))

(event EventSetFocused
  (Rendering|SetVisibility (Variables|Default|GetWidget) true false)
  (Utilities|FlowControl|RetriggerableDelay 0.1)
  (Rendering|SetVisibility (Variables|Default|GetWidget) false false))

(event EventInteract
  (params (InteractingActor :type Actor%20Object%20Reference)))

(event EventBeginPlay
  (CallFunction|SetupInteractionWidget))

(fn ConstructionScript)

(fn SetupInteractionWidget
  (if (Variables|Default|GetHasIneractName)
    (bind _aswb_interaction_feed_back (Utilities|Casting|CastToWB_InteractionFeedBack (UserInterface|GetWidget (Variables|Default|GetWidget))))
    (Default|UpdateWidget _aswb_interaction_feed_back (Variables|Default|GetInteract_Name))))

(fn OnRepIsTurn?
  (CallFunction|TurnActor))