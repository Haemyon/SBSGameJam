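; BP_Scaffolding2 is a pressure-plate style scaffold that triggers BP_Floor actors sharing its Tag.
; Box overlap begin calls FunctionInteract on each matching floor and plays a timeline moving the Scaffold along relative Z.
; Overlap end calls Second on those floors and plays a second timeline with negated Z.
; Interaction events are empty; OnRep IsTurn also calls TurnActor, but the logic setting IsTurn is disconnected.
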(event OnComponentBeginOverlap(Box)
  (params (OverlappedComponent :type Primitive%20Component%20Object%20Reference) (OtherActor :type Actor%20Object%20Reference) (OtherComp :type Primitive%20Component%20Object%20Reference) (OtherBodyIndex :type Integer) (bFromSweep :type Boolean) (SweepResult :type Hit%20Result%20Structure%20%28by%20ref%29))
  (bind _outactors (Actor|GetAllActorsOfClasswithTag "/Game/Blueprint/MAP1/BP_Floor.BP_Floor_C" (Variables|Default|GetTag)))
  (for _array_element _outactors
    (Default|FunctionInteract _array_element)
    (CallFunction|TurnActor)))

(event OnComponentEndOverlap(Box)
  (params (OverlappedComponent :type Primitive%20Component%20Object%20Reference) (OtherActor :type Actor%20Object%20Reference) (OtherComp :type Primitive%20Component%20Object%20Reference) (OtherBodyIndex :type Integer))
  (bind _outactors (Actor|GetAllActorsOfClasswithTag "/Game/Blueprint/MAP1/BP_Floor.BP_Floor_C" (Variables|Default|GetTag)))
  (for _array_element _outactors
    (Default|Second _array_element)
    (CallFunction|ReturnActor)))

(event Custom|TurnActor
  (bind _새_트랙_0 (Timeline|타임라인 PlayFromStart)
    (:Update
      (Transformation|SetRelativeLocation (Variables|Default|GetScaffold) (Math|Vector|MakeVector 0.0 0.0 _새_트랙_0) false false))))

(event Custom|ReturnActor
  (bind _새_트랙_0 (Timeline|타임라인_0 PlayFromStart)
    (:Update
      (Transformation|SetRelativeLocation (Variables|Default|GetScaffold) (Math|Vector|MakeVector 0.0 0.0 (* _새_트랙_0 -1.0)) false false))))

(event EventSetFocused)

(event EventInteract
  (params (InteractingActor :type Actor%20Object%20Reference)))

(event EventBeginPlay)

(fn ConstructionScript)

(fn SetupInteractionWidget)

(fn OnRepIsTurn?
  (CallFunction|TurnActor))

(fn OnRepDoorActor)

(fn OnRepArrayElement)