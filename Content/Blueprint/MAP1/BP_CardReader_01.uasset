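; BP_CardReader_01 is a MAP1 card reader that opens tagged double doors once the player has a key card.
; AddKeyCard raises the count and refreshes a feedback widget showing cards held out of one.
; SetFocused shows that widget and hides it after a short retriggerable delay.
; Interact, with enough cards, fires once, calling FunctionInteract on every BP_DoorDouble01 tagged DoubleDoor_01.
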(event Custom|AddKeyCard
  (Math|Float|IncrementFloat (Variables|Default|GetKeyCard)
    (:%20%20
      (CallFunction|SetupInteractionWidget))))

(event EventBeginPlay
  (CallFunction|SetupInteractionWidget))

(event EventSetFocused
  (Rendering|SetVisibility (Variables|Default|GetWidget) true false)
  (Utilities|FlowControl|RetriggerableDelay 0.1)
  (Rendering|SetVisibility (Variables|Default|GetWidget) false false))

(event EventInteract
  (params (InteractingActor :type Actor%20Object%20Reference))
  (if (>= (Variables|Default|GetKeyCard) 1.0)
    (Development|PrintString "Red_On")
    (if (not (Variables|Default|GetIs%20Turn?))
      (Variables|Default|SetIs%20Turn? true)
      (bind _outactors (Actor|GetAllActorsOfClasswithTag "/Game/Blueprint/MAP1/BP_DoorDouble01.BP_DoorDouble01_C" "DoubleDoor_01"))
      (for _array_element _outactors
        (Default|FunctionInteract _array_element)))))

(fn ConstructionScript)

(fn SetupInteractionWidget
  (bind _aswb_interaction_feed_back (Utilities|Casting|CastToWB_InteractionFeedBack (UserInterface|GetWidget (Variables|Default|GetWidget))))
  (Default|UpdateWidget _aswb_interaction_feed_back (Utilities|Text|ToText(String) (Utilities|String|Append "키 카드 " (Utilities|String|ToString(Integer) (Math|Float|Round (Variables|Default|GetKeyCard))) "/1"))))