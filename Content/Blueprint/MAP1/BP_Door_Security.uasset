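; BP_Door_Security is an interactable security trigger in MAP1 that opens or toggles a tagged door.
; Interacting once sets the replicated IsTurn flag, then finds BP_Door01 actors tagged Door1 and calls FunctionInteract on each.
; A widget shows the interaction name while focused and hides via a short retriggerable delay.
; The IsTurn replication handler calls TurnActor, which is currently empty.
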(event Custom|TurnActor)

(event EventSetFocused
  (Rendering|SetVisibility (Variables|Default|GetWidget) true false)
  (Utilities|FlowControl|RetriggerableDelay 0.1)
  (Rendering|SetVisibility (Variables|Default|GetWidget) false false))

(event EventInteract
  (params (InteractingActor :type Actor%20Object%20Reference))
  (if (not (Variables|Default|GetIsTurn?))
    (Variables|Default|SetIsTurn? true)
    (bind _outactors (Actor|GetAllActorsOfClasswithTag "/Game/Blueprint/MAP1/BP_Door01.BP_Door01_C" "Door1"))
    (for _array_element _outactors
      (bind _output_get (Variables|Default|SetDoorActor _array_element))
      (Default|FunctionInteract _output_get))))

(event EventBeginPlay
  (CallFunction|SetupInteractionWidget))

(fn ConstructionScript)

(fn SetupInteractionWidget
  (bind _aswb_interaction_feed_back (Utilities|Casting|CastToWB_InteractionFeedBack (UserInterface|GetWidget (Variables|Default|GetWidget))))
  (Default|UpdateWidget _aswb_interaction_feed_back (Variables|Default|GetInteract_Name)))

(fn OnRepIsTurn?
  (CallFunction|TurnActor))

(fn OnRepDoorActor)