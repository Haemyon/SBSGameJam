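; BP_Lever2 is a one-shot interactable lever that triggers every BP_Door04 carrying a matching tag.
; Interact sets IsTurn, calls each matching door's interact function, and plays a timeline that rolls the lever.
; IsTurn's RepNotify also plays the turn, keeping the animation in step with replicated state.
; Focus shows a named interaction widget, which a short retriggerable delay hides once focus stops refreshing.
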(event Custom|TurnActor
  (bind _새_트랙_0 (Timeline|타임라인 Play)
    (:Update
      (Transformation|SetRelativeRotation (Variables|Default|GetScene) (Math|Rotator|MakeRotator _새_트랙_0 0.0 0.0) false false))))

(event EventSetFocused
  (Rendering|SetVisibility (Variables|Default|GetWidget) true false)
  (Utilities|FlowControl|RetriggerableDelay 0.1)
  (Rendering|SetVisibility (Variables|Default|GetWidget) false false))

(event EventInteract
  (params (InteractingActor :type Actor%20Object%20Reference))
  (if (not (Variables|Default|GetIsTurn?))
    (Variables|Default|SetIsTurn? true)
    (bind _outactors (Actor|GetAllActorsOfClasswithTag "/Game/Blueprint/MAP1/BP_Door04.BP_Door04_C" (Variables|Default|GetTag)))
    (for _array_element _outactors
      (Default|FunctionInteract _array_element)
      (CallFunction|TurnActor))))

(event EventBeginPlay
  (CallFunction|SetupInteractionWidget))

(fn ConstructionScript)

(fn SetupInteractionWidget
  (bind _aswb_interaction_feed_back (Utilities|Casting|CastToWB_InteractionFeedBack (UserInterface|GetWidget (Variables|Default|GetWidget))))
  (Default|UpdateWidget _aswb_interaction_feed_back (Variables|Default|GetInteract_Name)))

(fn OnRepIsTurn?
  (CallFunction|TurnActor))

(fn OnRepDoorActor)