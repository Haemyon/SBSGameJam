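; BP_Door04 is an interactable door that moves once along Z, with no path to reset it.
; FunctionInteract sets IsTurn on first use and calls TurnActor, whose Turn timeline drives the Scene component's relative Z location.
; IsTurn has an OnRep handler that also calls TurnActor, replicating the motion.
; Interact and SetFocused are empty, and the interaction-widget label and visibility logic is disconnected.
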(event Custom|TurnActor
  (bind _z (Timeline|Turn Play)
    (:Update
      (Transformation|SetRelativeLocation (Variables|Default|GetScene) (Math|Vector|MakeVector 0.0 0.0 _z) false false))))

(event EventFunctionInteract
  (if (not (Variables|Default|GetIsTurn?))
    (Variables|Default|SetIsTurn? true)
    (CallFunction|TurnActor)))

(event EventSetFocused)

(event EventInteract
  (params (InteractingActor :type Actor%20Object%20Reference)))

(event EventBeginPlay)

(fn ConstructionScript)

(fn SetupInteractionWidget
  (if (Variables|Default|GetHasIneractName)
    (bind _aswb_interaction_feed_back (Utilities|Casting|CastToWB_InteractionFeedBack (UserInterface|GetWidget (Variables|Default|GetWidget))))
    (Default|UpdateWidget _aswb_interaction_feed_back (Variables|Default|GetInteract_Name))))

(fn OnRepIsTurn?
  (CallFunction|TurnActor))