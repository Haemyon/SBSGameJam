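; BP_Door03 is a MAP1 door that opens by moving vertically once its interaction function has been called at least twice, apparently for generators.
; FunctionInteract increments GenOnCount and sets IsTurn at the threshold, whose OnRep calls TurnActor.
; TurnActor plays the Turn timeline, adding its Z value to the Cube's relative location on every update, so movement accumulates.
; Interact, focus and generator events are empty, and the widget visibility logic is disconnected.
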(event Custom|TurnActor
  (bind _cube (Variables|Default|GetCube))
  (bind _relativelocation (Variables|/Script/Engine.SceneComponent|GetRelativeLocation _cube))
  (bind _z (Timeline|Turn PlayFromStart)
    (:Update
      (Transformation|SetRelativeLocation _cube (Math|Vector|MakeVector (.x _relativelocation) (.y _relativelocation) (+ (.z _relativelocation) _z)) false false))))

(event Custom|Genrator_On)

(event EventFunctionInteract
  (bind _result (Math|Float|IncrementFloat (Variables|Default|GetGenOnCount))
    (:%20%20
      (bind _output_get (Variables|Default|SetGenOnCount _result))
      (if (>= (Variables|Default|GetGenOnCount) 2.0)
        (if (not (Variables|Default|GetIsTurn?))
          (Variables|Default|SetIsTurn? true))))))

(event EventSetFocused)

(event EventInteract
  (params (InteractingActor :type Actor%20Object%20Reference)))

(fn ConstructionScript)

(fn SetupInteractionWidget
  (bind _aswb_interaction_feed_back (Utilities|Casting|CastToWB_InteractionFeedBack (UserInterface|GetWidget (Variables|Default|GetWidget))))
  (Default|UpdateWidget _aswb_interaction_feed_back (Variables|Default|GetInteract_Name)))

(fn OnRepIsTurn?
  (CallFunction|TurnActor))