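; Interactable two-panel elevator door that opens or slides once, with an on-screen prompt showing its interact name.
; Interact sets IsTurn a single time, and its RepNotify plays the Turn timeline.
; Each timeline update adds its Z value to the panels' current X positions in opposite directions, so movement accumulates per tick.
; SetFocused shows the prompt widget and uses a retriggerable delay to hide it once focus calls stop.
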(event Custom|TurnActor
  (bind _cube (Variables|Default|GetCube))
  (bind _cube1 (Variables|Default|GetCube1))
  (bind _relativelocation (Variables|/Script/Engine.SceneComponent|GetRelativeLocation _cube))
  (bind _relativelocation_2 (Variables|/Script/Engine.SceneComponent|GetRelativeLocation _cube1))
  (bind _z (Timeline|Turn PlayFromStart)
    (:Update
      (Transformation|SetRelativeLocation _cube1 (Math|Vector|MakeVector (+ (.x _relativelocation_2) _z) (.y _relativelocation_2) (.z _relativelocation_2)) false false)
      (Transformation|SetRelativeLocation _cube (Math|Vector|MakeVector (- (.x _relativelocation) _z) (.y _relativelocation) (.z _relativelocation)) false false))))

(event EventSetFocused
  (Rendering|SetVisibility (Variables|Default|GetWidget) true false)
  (Utilities|FlowControl|RetriggerableDelay 0.1)
  (Rendering|SetVisibility (Variables|Default|GetWidget) false false))

(event EventInteract
  (params (InteractingActor :type Actor%20Object%20Reference))
  (if (not (Variables|Default|GetIsTurn?))
    (Variables|Default|SetIsTurn? true)))

(event EventBeginPlay
  (CallFunction|SetupInteractionWidget))

(fn ConstructionScript)

(fn SetupInteractionWidget
  (bind _aswb_interaction_feed_back (Utilities|Casting|CastToWB_InteractionFeedBack (UserInterface|GetWidget (Variables|Default|GetWidget))))
  (Default|UpdateWidget _aswb_interaction_feed_back (Variables|Default|GetInteract_Name)))

(fn OnRepIsTurn?
  (CallFunction|TurnActor))