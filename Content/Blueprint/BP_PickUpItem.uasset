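; BP_PickUpItem is a world pickup item that hands its ItemID to whoever interacts with it, then destroys itself.
; The construction script looks up the ID in DT_Item to set the mesh, scale, name and prompt height.
; On BeginPlay the name is pushed into a WB_InteractionFeedBack widget.
; SetFocused shows that widget, with a retriggerable delay hiding it shortly after focus calls stop.
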(event EventBeginPlay
  (CallFunction|SetupInteractionWidget))

(event EventInteract
  (params (InteractingActor :type Actor%20Object%20Reference))
  (Class|BPITools|HandlePickUp(Message) InteractingActor (Variables|Default|GetItemID))
  (Actor|DestroyActor))

(event EventSetFocused
  (Rendering|SetVisibility (Variables|Default|GetWidget) true false)
  (Utilities|FlowControl|RetriggerableDelay 0.1)
  (Rendering|SetVisibility (Variables|Default|GetWidget) false false))

(fn ConstructionScript
  (bind _staticmesh (Variables|Default|GetStaticMesh))
  (bind _widget (Variables|Default|GetWidget))
  (bind _returnvalue (Transformation|GetRelativeTransform _widget))
  (bind _returnvalue_2 (Transformation|GetRelativeTransform _staticmesh))
  (bind _returnvalue_3 (Utilities|GetDataTableRow "/Game/Blueprint/DATA/DT_Item.DT_Item" (Utilities|String|StringToName (Variables|Default|GetItemID)))
    (:then
      (Components|StaticMesh|SetStaticMesh _staticmesh (.SM_Item (Utilities|Struct|BreakS_Item _returnvalue_3)))
      (Transformation|SetRelativeTransform _staticmesh (Math|Transform|MakeTransform (.location _returnvalue_2) (.rotation _returnvalue_2) (Math|Conversions|ToVector(Float) (.MultiplySIze (Utilities|Struct|BreakS_Item _returnvalue_3)))) false false)
      (Variables|Default|SetName (.Name (Utilities|Struct|BreakS_Item _returnvalue_3)))
      (Transformation|SetRelativeTransform _widget (Math|Transform|MakeTransform (Math|Vector|MakeVector (.x (.location _returnvalue)) (.y (.location _returnvalue)) (.WidgetLocation_Z (Utilities|Struct|BreakS_Item _returnvalue_3))) (.rotation _returnvalue) (.scale _returnvalue)) false false))))

(fn SetupInteractionWidget
  (bind _aswb_interaction_feed_back (Utilities|Casting|CastToWB_InteractionFeedBack (UserInterface|GetWidget (Variables|Default|GetWidget))))
  (Default|UpdateWidget _aswb_interaction_feed_back (Utilities|Text|ToText(String) (Variables|Default|GetName))))