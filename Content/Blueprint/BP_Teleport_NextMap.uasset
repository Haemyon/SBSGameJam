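; BP_Teleport_NextMap is a trigger volume that teleports all characters to a fixed destination area once enough overlaps accumulate.
; Box begin and end overlaps raise and lower PlayerCount, printing it each time, with no filter on what overlaps.
; At four or more, Teleport moves every BP_CoreCharacter to a random spot in hard-coded coordinate ranges, without loading another level.
; PlayerCount has an empty OnRep function.
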(event OnComponentBeginOverlap(Box)
  (params (OverlappedComponent :type Primitive%20Component%20Object%20Reference) (OtherActor :type Actor%20Object%20Reference) (OtherComp :type Primitive%20Component%20Object%20Reference) (OtherBodyIndex :type Integer) (bFromSweep :type Boolean) (SweepResult :type Hit%20Result%20Structure%20%28by%20ref%29))
  (bind _result (Math|Float|IncrementFloat (Variables|Default|GetPlayerCount))
    (:%20%20
      (bind _output_get (Variables|Default|SetPlayerCount _result))
      (Development|PrintString (Utilities|String|ToString(Float) _output_get))
      (if (>= (Variables|Default|GetPlayerCount) 4.0)
        (CallFunction|Teleport)))))

(event OnComponentEndOverlap(Box)
  (params (OverlappedComponent :type Primitive%20Component%20Object%20Reference) (OtherActor :type Actor%20Object%20Reference) (OtherComp :type Primitive%20Component%20Object%20Reference) (OtherBodyIndex :type Integer))
  (bind _result (Math|Float|DecrementFloat (Variables|Default|GetPlayerCount))
    (:%20%20
      (bind _output_get (Variables|Default|SetPlayerCount _result))
      (Development|PrintString (Utilities|String|ToString(Float) _output_get)))))

(event Custom|Teleport
  (bind _outactors (Actor|GetAllActorsOfClass "/Game/Player/BP_CoreCharacter.BP_CoreCharacter_C"))
  (for _array_element _outactors
    (Transformation|SetActorLocation _array_element (Math|Vector|MakeVector (Math|Random|RandomFloatinRange -2.9e+03 -3.1e+03) (Math|Random|RandomFloatinRange 8.18e+03 8.3e+03) 6e+01) false false)))

(fn ConstructionScript)

(fn OnRepPlayerCount)