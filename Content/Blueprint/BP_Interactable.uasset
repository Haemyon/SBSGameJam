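; Interactable actor that shows a named interaction prompt and rotates its cube once when used.
; On BeginPlay it passes the interact name to its WB_InteractionFeedBack widget.
; SetFocused shows the widget, and a short retriggerable delay hides it once focus calls stop.
; Interact sets IsTurn only if unset, and its RepNotify plays the Turn timeline that drives the cube's yaw.
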(event Custom|TurnActor
  (bind _z (Timeline|Turn PlayFromStart)
    (:Update
      (Transformation|SetRelativeRotation (Variables|Default|GetCube) (Math|Rotator|MakeRotator 0.0 0.0 _z) false false))))

(event EventSetFocused
  (Rendering|SetVisibility (Variables|Default|GetWidget) true false)
  (Utilities|FlowControl|RetriggerableDelay 0.1)
  (Rendering|SetVisibility (Variables|Default|GetWidget) false false))

(event EventInteract
  (params (InteractingActor :type Actor%20Object%20Reference))
  (if (not (Variables|Default|GetIsTurn?))
    (Variables|Default|SetIsTurn? true)))

(event EventBeginPlay
  (CallFunction|SetupInteractionWidget))

(fn ConstructionScript)

(fn SetupInteractionWidget
  (bind _aswb_interaction_feed_back (Utilities|Casting|CastToWB_InteractionFeedBack (UserInterface|GetWidget (Variables|Default|GetWidget))))
  (Default|UpdateWidget _aswb_interaction_feed_back (Variables|Default|GetInteract_Name)))

(fn OnRepIsTurn?
  (CallFunction|TurnActor))