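; BP_CoreWeapon is a base weapon actor that takes its appearance from the item data table and responds to a character's primary action.
; On SetupActor, it looks up its ItemID row in DT_Item to set its static mesh, then binds to the owning BPCoreCharacter's OnPrimaryAction event.
; The primary action forwards to an empty HandlePrimaryAction hook, apparently left for child weapons to implement.
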(event Custom|PrimaryAction
  (CallFunction|HandlePrimaryAction))

(event Custom|SetupActor
  (CallFunction|Setup)
  (EventDispatchers|BindEventtoOnPrimaryAction (Variables|Default|GetAs%20BP%20Core%20Character) (delegate Custom|PrimaryAction)))

(event Custom|Handle_PrimaryAction)

(fn ConstructionScript)

(fn Setup
  (bind _returnvalue (Utilities|GetDataTableRow "/Game/Blueprint/DATA/DT_Item.DT_Item" (Utilities|String|StringToName (Variables|Default|GetItemID)))
    (:then
      (Components|StaticMesh|SetStaticMesh (Variables|Default|GetStaticMesh) (.SM_Item (Utilities|Struct|BreakS_Item _returnvalue))))))